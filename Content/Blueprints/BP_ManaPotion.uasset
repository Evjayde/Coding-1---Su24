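; BP_ManaPotion is a holdable mana potion that offers itself to BP_ThirdPersonCharacterCustom when the character overlaps its PickupTrigger.
; Drop detaches the root and enables physics and collision on Neck, while Pickup is empty and its hand-socket attach is left unwired.
; Primary action prints a +10 mana message without changing any mana value, clears the character's HeldItem and destroys the potion.
; Secondary action only prints a placeholder message.
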(event OnComponentBeginOverlap(PickupTrigger)
  (params (OverlappedComponent :type Primitive%20Component%20Object%20Reference) (OtherActor :type Actor%20Object%20Reference) (OtherComp :type Primitive%20Component%20Object%20Reference) (OtherBodyIndex :type Integer) (bFromSweep :type Boolean) (SweepResult :type Hit%20Result%20Structure%20%28by%20ref%29))
  (bind _asbp_third_person_character_custom (Utilities|Casting|CastToBP_ThirdPersonCharacterCustom OtherActor))
  (Default|TrytoPickUp _asbp_third_person_character_custom self))

(event EventSecondaryAction
  (Development|PrintString "This is your secondary action!"))

(event EventPrimaryAction
  (params (ref_ThirdPersonCharCustom :type BP%20Third%20Person%20Character%20Custom%20Object%20Reference))
  ;[0.2686 0.3473 0.7934] Use Potion & Gain Mana
  (Development|PrintString "You gained +10 mana!" true true "(R=0.054306,G=0.026895,B=0.793403,A=1.000000)")
  (Variables|/Game/Blueprints/BP_ThirdPersonCharacterCustom.BP_ThirdPersonCharacterCustom_C|SetHeldItem ref_ThirdPersonCharCustom 0)
  (Actor|DestroyActor))

(event EventDrop
  (Transformation|DetachFromComponent (Variables|Default|GetDefaultSceneRoot) "KeepRelative" "KeepRelative" "KeepRelative" true)
  (Physics|SetSimulatePhysics (Variables|Default|GetNeck) true)
  (Collision|SetCollisionEnabled (Variables|Default|GetNeck) "QueryAndPhysics"))

(event EventPickup
  (params (ParentMesh :type Skeletal%20Mesh%20Component%20Object%20Reference)))

(fn ConstructionScript)