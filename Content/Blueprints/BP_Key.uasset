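; BP_Key is a collectible key pickup for the player character.
; When its box collision overlaps an actor, it casts to BP_ThirdPersonCharacterCustom, increments that character's KeyCount and destroys itself.
; Debug strings print on spawn, on pickup with the new count, and when the cast fails.
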(event OnComponentBeginOverlap(BoxCollision)
  (params (OverlappedComponent :type Primitive%20Component%20Object%20Reference) (OtherActor :type Actor%20Object%20Reference) (OtherComp :type Primitive%20Component%20Object%20Reference) (OtherBodyIndex :type Integer) (bFromSweep :type Boolean) (SweepResult :type Hit%20Result%20Structure%20%28by%20ref%29))
  (bind _asbp_third_person_character_custom (Utilities|Casting|CastToBP_ThirdPersonCharacterCustom OtherActor)
    (:then
      (Development|PrintString "A Player ran into me!" true true "(R=0.000000,G=0.660000,B=1.000000,A=1.000000)" 5.0)
      (Variables|/Game/Blueprints/BP_ThirdPersonCharacterCustom.BP_ThirdPersonCharacterCustom_C|SetKeyCount _asbp_third_person_character_custom (+ (Variables|/Game/Blueprints/BP_ThirdPersonCharacterCustom.BP_ThirdPersonCharacterCustom_C|GetKeyCount _asbp_third_person_character_custom) 1))
      (Development|PrintString (Utilities|String|Append "The Player has " (Utilities|String|ToString(Integer) (Variables|/Game/Blueprints/BP_ThirdPersonCharacterCustom.BP_ThirdPersonCharacterCustom_C|GetKeyCount _asbp_third_person_character_custom)) " keys!"))
      (Actor|DestroyActor))
    (:CastFailed
      (Development|PrintString "Key player cast failed" true true "(R=1.000000,G=0.082091,B=0.221944,A=1.000000)"))))

(event EventBeginPlay
  (Development|PrintString "This key exists!" true true "(R=0.223958,G=0.000000,B=0.447917,A=1.000000)"))

(fn ConstructionScript)